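; BP_WinnerHighlight is a GM1 game-mode actor that marks the current leading player with a particle effect.
; When GM_GM1 signals game start, it assigns the highlight effect from LeaderFXData, hides it, and starts a looping timer at that data's refresh rate.
; The timer polls the game mode for the winner and shows the effect when that changes.
; Tick moves the actor to the tracked player's location with sweep enabled.
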(event `self.ReceiveBeginPlay`
  (bind _asgm_gm1 (cast `/Game/Systems/Blueprints/GM1/Systems/GM_GM1` (`GameplayStatics.GetGameMode`)))
  (add `/Game/Systems/Blueprints/GM1/Systems/GM_GM1.GameStarted` _asgm_gm1 (delegate `StartFollow`)))

(event `StartFollow`
  (bind _leaderfxdata (`self.LeaderFXData`))
  (`KismetSystemLibrary.K2_SetTimerDelegate` (delegate `UpdateTrackedPlayer`) (`/Game/Systems/Blueprints/GM1/Data/PDA_LeaderFX_GM1.refreshRate` _leaderfxdata) true)
  (`NiagaraComponent.SetAsset` (`self.Particles`) (`/Game/Systems/Blueprints/GM1/Data/PDA_LeaderFX_GM1.HighlightFX` _leaderfxdata) false)
  (`SceneComponent.SetVisibility` (`self.Particles`) false false))

(event `UpdateTrackedPlayer`
  (bind _asgm_gm1 (cast `/Game/Systems/Blueprints/GM1/Systems/GM_GM1` (`GameplayStatics.GetGameMode`)))
  (bind _player (`/Game/Systems/Blueprints/GM1/Systems/GM_GM1.GetCurrentWinnerInfo` _asgm_gm1))
  (if (!= _player (`self.trackedPlayer`))
    (set `self.trackedPlayer` _player)
    (`SceneComponent.SetVisibility` (`self.Particles`) true false)))

(event `self.ReceiveTick`
  (params (DeltaSeconds :type "Float (single-precision)"))
  (bind _trackedplayer (`self.trackedPlayer`))
  (if (`KismetSystemLibrary.IsValid` _trackedplayer)
    (`self.K2_SetActorLocation` (`self.K2_GetActorLocation` _trackedplayer) true)))

(fn `UserConstructionScript`)