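; Hazard timer for GM1 that fires timed meteor pattern, meteor shower, bumper, arena tilt/ice ring and wall events.
; Construction picks a random or indexed schedule from ScheduleData; StartSchedule sorts all schedules by event time and starts the clock.
; While playing, Tick advances an index per hazard track, triggering all due events with an FX alert on spawners, bumpers, arena or walls.
; LowerWalls is an empty stub.
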(event `self.ReceiveTick`
  (params (DeltaSeconds :type "Float (single-precision)"))
  (if (`self.IsPlaying`)
    (`/Game/Systems/Blueprints/GM1/Libraries/GM1_MacroLib.PlusEqualsFloat` (`self.currentTime`) DeltaSeconds
      (:`  `
        (`self.AdvanceArenaHazardEvents`)
        (`self.AdvanceMeteorPatternEvents`)
        (`self.AdvanceMeteorShowerEvents`)
        (`self.AdvanceBumperEvents`)
        (`self.AdvanceWallEvents`)))))

(event `RaiseWalls`
  (params (walls :type "Array of SkeletalMeshActor Object Reference") (timer :type "Float (double-precision)"))
  (`KismetSystemLibrary.Delay` timer)
  (for _array_element walls
    (`SkeletalMeshComponent.PlayAnimation` (`SkeletalMeshActor.SkeletalMeshComponent` _array_element) "/Game/GameMode1/Art/EnviormentAssets/Barrier/Animations/Barrier_FallDown.Barrier_FallDown" false)
    (`GameplayStatics.PlaySound2D` "/Game/Audio/Placeholder/Q_WallLift.Q_WallLift" 1.0 1.0 0.0 null null)))

(event `LowerWalls`
  (params (walls :type "Array of SkeletalMeshActor Object Reference")))

(fn `Activate Arena Hazard Event`
  (params (hazardEvent :type "/Game/Systems/Blueprints/GM1/Hazards/HazardTimer/Data/Events/F_ArenaHazardEvent Structure"))
  (bind (_eventtime _eventtype _play _tiltsettings _iceringsettings) (break `/Game/Systems/Blueprints/GM1/Hazards/HazardTimer/Data/Events/F_ArenaHazardEvent` hazardEvent))
  (bind _asgm_gm1 (cast `/Game/Systems/Blueprints/GM1/Systems/GM_GM1` (`GameplayStatics.GetGameMode`)))
  (`/Game/Systems/Blueprints/BP_FXEventManager.GM1_HazardSpawnAlert` (`/Game/Systems/Blueprints/GM1/Systems/GM_GM1.FXManager` _asgm_gm1))
  (switch `/Game/Systems/Blueprints/GM1/Hazards/HazardTimer/Data/E_ArenaHazardType` _eventtype
    (:`NewEnumerator0`
      ;[0 0.08452 1 0.5] Start/Stop Arena Tilt
      (bind _returnvalue (`GameplayStatics.GetActorOfClass` "/Game/Systems/Blueprints/GM1/Hazards/BP_Arena.BP_Arena_C"))
      (if _play
        (set `/Game/Systems/Blueprints/GM1/Hazards/BP_Arena.ArenaTiltData` _tiltsettings _returnvalue)
        (`/Game/Systems/Blueprints/GM1/Hazards/BP_Arena.StartTilt` _returnvalue)
        (else
          (`/Game/Systems/Blueprints/GM1/Hazards/BP_Arena.StopTilt` _returnvalue))))
    (:`NewEnumerator1`
      ;[0.1536 0 1 0.5] Play/Pause Ice Ring Growth
      (bind _returnvalue_2 (`GameplayStatics.GetActorOfClass` "/Game/Systems/Blueprints/GM1/Hazards/BP_Arena.BP_Arena_C"))
      (if _play
        (set `/Game/Systems/Blueprints/GM1/Hazards/BP_Arena.IceRingData` _iceringsettings _returnvalue_2)
        (`/Game/Systems/Blueprints/GM1/Hazards/BP_Arena.Start Ice Grow` _returnvalue_2)
        (else
          (`/Game/Systems/Blueprints/GM1/Hazards/BP_Arena.Stop Ice Grow` _returnvalue_2))))))

(fn `Activate Bumper Event`
  (params (hazardEvent :type "/Game/Systems/Blueprints/GM1/Hazards/HazardTimer/Data/Events/F_BumperEvent Structure"))
  (bind (_eventtime _bumpers _raise) (break `/Game/Systems/Blueprints/GM1/Hazards/HazardTimer/Data/Events/F_BumperEvent` hazardEvent))
  (bind _asgm_gm1 (cast `/Game/Systems/Blueprints/GM1/Systems/GM_GM1` (`GameplayStatics.GetGameMode`)))
  (`/Game/Systems/Blueprints/BP_FXEventManager.GM1_HazardSpawnAlert` (`/Game/Systems/Blueprints/GM1/Systems/GM_GM1.FXManager` _asgm_gm1))
  (if _raise
    (for _array_element _bumpers
      (`/Game/Systems/Blueprints/GM1/Hazards/BP_Bumper.RaiseBumper` _array_element))
    (else
      (for _array_element_2 _bumpers
        (`/Game/Systems/Blueprints/GM1/Hazards/BP_Bumper.LowerBumper` _array_element_2)))))

(fn `Activate Meteor Pattern Event`
  (params (hazardEvent :type "/Game/Systems/Blueprints/GM1/Hazards/HazardTimer/Data/Events/F_MeteorPatternEvent Structure"))
  (locals (spawner :type "/Game/Systems/Blueprints/GM1/Hazards/Meteors/BP_GM1_MeteorSpawner Object Reference"))
  (bind (_eventtime _pattern _spawner) (break `/Game/Systems/Blueprints/GM1/Hazards/HazardTimer/Data/Events/F_MeteorPatternEvent` hazardEvent))
  (bind (_eventtime_2 _pattern_2 _spawner_2 _basicmeteorsettings _position _lineorigin _linedestination _ringburstradius _lineringburstpoints) (break `/Game/Systems/Blueprints/GM1/Hazards/HazardTimer/Data/Events/F_MeteorPatternEvent` (`local.hazardEvent`)))
  (bind (_eventtime_3 _pattern_3 _spawner_3 _basicmeteorsettings_2 _position_2) (break `/Game/Systems/Blueprints/GM1/Hazards/HazardTimer/Data/Events/F_MeteorPatternEvent` (`local.hazardEvent`)))
  (bind (_eventtime_4 _pattern_4 _spawner_4 _basicmeteorsettings_3 _position_3 _lineorigin_2 _linedestination_2 _ringburstradius_2 _lineringburstpoints_2) (break `/Game/Systems/Blueprints/GM1/Hazards/HazardTimer/Data/Events/F_MeteorPatternEvent` (`local.hazardEvent`)))
  (bind (_eventtime_5 _pattern_5 _spawner_5 _basicmeteorsettings_4 _position_4 _lineorigin_3 _linedestination_3 _ringburstradius_3 _lineringburstpoints_3) (break `/Game/Systems/Blueprints/GM1/Hazards/HazardTimer/Data/Events/F_MeteorPatternEvent` (`local.hazardEvent`)))
  (bind _asgm_gm1 (cast `/Game/Systems/Blueprints/GM1/Systems/GM_GM1` (`GameplayStatics.GetGameMode`)))
  (`/Game/Systems/Blueprints/BP_FXEventManager.GM1_HazardSpawnAlert` (`/Game/Systems/Blueprints/GM1/Systems/GM_GM1.FXManager` _asgm_gm1))
  (`/Engine/EditorBlueprintResources/StandardMacros.IsValid` _spawner
    (:`Is Valid`
      (set `local.spawner` _spawner))
    (:`Is Not Valid`
      (bind _spawner_6 (`self.Get Valid Meteor Spawner`))
      (set `local.spawner` _spawner_6)))
  (switch `/Game/Systems/Blueprints/GM1/Hazards/HazardTimer/Data/E_MeteorPatternType` _pattern
    (:`NewEnumerator0`
      ;[0.4241 0 1 0.5] Single Meteor
      (`/Game/Systems/Blueprints/GM1/Hazards/Meteors/BP_GM1_MeteorSpawner.Spawn Meteor Single` (`local.spawner`) _basicmeteorsettings_2 _position_2))
    (:`NewEnumerator1`
      ;[0 0.08929 1 0.5] Meteor Line
      (`/Game/Systems/Blueprints/GM1/Hazards/Meteors/BP_GM1_MeteorSpawner.Spawn Meteor Line` (`local.spawner`) _basicmeteorsettings_3 _lineorigin_2 _linedestination_2 _lineringburstpoints_2))
    (:`NewEnumerator2`
      ;[0 0.505 0.5816 0.5] Meteor Ring
      (`/Game/Systems/Blueprints/GM1/Hazards/Meteors/BP_GM1_MeteorSpawner.Spawn Meteor Ring` (`local.spawner`) _basicmeteorsettings_4 _position_4 _ringburstradius_3 _lineringburstpoints_3))
    (:`NewEnumerator3`
      ;[0.00612 0.3663 0 0.5] Meteor Burst
      (`/Game/Systems/Blueprints/GM1/Hazards/Meteors/BP_GM1_MeteorSpawner.Spawn Meteor Burst` (`local.spawner`) _basicmeteorsettings _position _ringburstradius _lineringburstpoints))))

(fn `Activate Meteor Shower Event`
  (params (hazardEvent :type "/Game/Systems/Blueprints/GM1/Hazards/HazardTimer/Data/Events/F_MeteorShowerEvent Structure"))
  (locals (spawner :type "/Game/Systems/Blueprints/GM1/Hazards/Meteors/BP_GM1_MeteorSpawner Object Reference"))
  (bind (_eventtime _spawner _play _settings) (break `/Game/Systems/Blueprints/GM1/Hazards/HazardTimer/Data/Events/F_MeteorShowerEvent` hazardEvent))
  (bind _spawner_2 (`local.spawner`))
  (bind _asgm_gm1 (cast `/Game/Systems/Blueprints/GM1/Systems/GM_GM1` (`GameplayStatics.GetGameMode`)))
  (`/Game/Systems/Blueprints/BP_FXEventManager.GM1_HazardSpawnAlert` (`/Game/Systems/Blueprints/GM1/Systems/GM_GM1.FXManager` _asgm_gm1))
  (if _play
    (`/Engine/EditorBlueprintResources/StandardMacros.IsValid` _spawner
      (:`Is Valid`
        (set `local.spawner` _spawner))
      (:`Is Not Valid`
        (bind _returnvalue (`|SpawnActorFromClass` "/Game/Systems/Blueprints/GM1/Hazards/Meteors/BP_GM1_MeteorSpawner.BP_GM1_MeteorSpawner_C" (`KismetMathLibrary.MakeTransform` (0.0 0.0 25.0)) "Undefined" "MultiplyWithRoot" null _settings null))
        (set `local.spawner` _returnvalue)))
    (set `/Game/Systems/Blueprints/GM1/Hazards/Meteors/BP_GM1_MeteorSpawner.Data` _settings _spawner_2)
    (`/Game/Systems/Blueprints/GM1/Hazards/Meteors/BP_GM1_MeteorSpawner.Start Spawn` _spawner_2)
    (else
      (`/Engine/EditorBlueprintResources/StandardMacros.IsValid` _spawner
        (:`Is Valid`
          (`/Game/Systems/Blueprints/GM1/Hazards/Meteors/BP_GM1_MeteorSpawner.Stop Spawn` _spawner))
        (:`Is Not Valid`
          (bind _outactors (`GameplayStatics.GetAllActorsOfClass` "/Game/Systems/Blueprints/GM1/Hazards/Meteors/BP_GM1_MeteorSpawner.BP_GM1_MeteorSpawner_C"))
          (for _array_element _outactors
            (`/Game/Systems/Blueprints/GM1/Hazards/Meteors/BP_GM1_MeteorSpawner.Stop Spawn` _array_element)))))))

(fn `Activate Wall Event`
  (params (hazardEvent :type "/Game/Systems/Blueprints/GM1/Hazards/HazardTimer/Data/Events/F_WallHazardEvent Structure"))
  (bind (_eventtime _walls _raise) (break `/Game/Systems/Blueprints/GM1/Hazards/HazardTimer/Data/Events/F_WallHazardEvent` hazardEvent))
  (bind (_eventtime_2 _walls_2 _raise_2 _heads_up) (break `/Game/Systems/Blueprints/GM1/Hazards/HazardTimer/Data/Events/F_WallHazardEvent` (`local.hazardEvent`)))
  (bind _asgm_gm1 (cast `/Game/Systems/Blueprints/GM1/Systems/GM_GM1` (`GameplayStatics.GetGameMode`)))
  (`/Game/Systems/Blueprints/BP_FXEventManager.GM1_HazardSpawnAlert` (`/Game/Systems/Blueprints/GM1/Systems/GM_GM1.FXManager` _asgm_gm1))
  (for _array_element _walls
    (bind _skeletalmeshcomponent (`SkeletalMeshActor.SkeletalMeshComponent` _array_element))
    (bind _returnvalue (`PrimitiveComponent.CreateDynamicMaterialInstance` _skeletalmeshcomponent 2 "/Game/GameMode1/Art/Materials/MI_OverlayGlow.MI_OverlayGlow" "OverlayGlow"))
    (`PrimitiveComponent.SetMaterial` _skeletalmeshcomponent 2 _returnvalue))
  (bind _asgm_gm1_2 (cast `/Game/Systems/Blueprints/GM1/Systems/GM_GM1` (`GameplayStatics.GetGameMode`)))
  (if _raise
    (`self.RaiseWalls` _walls_2 _heads_up)
    (bind _fxmanager (`/Game/Systems/Blueprints/GM1/Systems/GM_GM1.FXManager` _asgm_gm1_2))
    (`/Game/Systems/Blueprints/BP_FXEventManager.GM1_WallsRemoved` _fxmanager _walls_2)
    (else
      (`self.LowerWalls` _walls_2)
      (`/Game/Systems/Blueprints/BP_FXEventManager.GM1_WallsReplaced` _fxmanager _walls_2))))

(fn `AdvanceArenaHazardEvents`
  (bind (_meteorpatternschedule _meteorshowerschedule _bumperschedule _arenahazardschedule) (break `/Game/Systems/Blueprints/GM1/Hazards/HazardTimer/Data/F_HazardSchedule` (`self.activeSchedule`)))
  (bind _returnvalue (`KismetArrayLibrary.Array_Length` _arenahazardschedule))
  (bind _returnvalue_2 (< (`self.currentArenaHazardEvent`) _returnvalue))
  (bind _output (`|GetArrayItem` _arenahazardschedule (`KismetMathLibrary.Clamp` (`self.currentArenaHazardEvent`) 0 (- _returnvalue 1))))
  (if _returnvalue_2
    ;[0 0 0 0.5] While loop ensures that multiple events scheduled for the same time will trigger on the same frame. Take care not to start too many (>10) events at the same time, though.
    (while (and _returnvalue_2 (<= (`.EventTime_26_97FD4C2C4CD31F34555A7AA230F32490` (break `/Game/Systems/Blueprints/GM1/Hazards/HazardTimer/Data/Events/F_ArenaHazardEvent` _output)) (`self.currentTime`)))
      (`self.Activate Arena Hazard Event` _output)
      (`/Engine/EditorBlueprintResources/StandardMacros.IncrementInt` (`self.currentArenaHazardEvent`)))))

(fn `AdvanceBumperEvents`
  (bind (_meteorpatternschedule _meteorshowerschedule _bumperschedule) (break `/Game/Systems/Blueprints/GM1/Hazards/HazardTimer/Data/F_HazardSchedule` (`self.activeSchedule`)))
  (bind _returnvalue (`KismetArrayLibrary.Array_Length` _bumperschedule))
  (bind _returnvalue_2 (< (`self.currentBumperEvent`) _returnvalue))
  (bind _output (`|GetArrayItem` _bumperschedule (`KismetMathLibrary.Clamp` (`self.currentBumperEvent`) 0 (- _returnvalue 1))))
  (if _returnvalue_2
    ;[0 0 0 0.5] While loop ensures that multiple events scheduled for the same time will trigger on the same frame. Take care not to start too many (>10) events at the same time, though.
    (while (and _returnvalue_2 (<= (`.EventTime_10_4C73EC23445F080D0654368106218ACC` (break `/Game/Systems/Blueprints/GM1/Hazards/HazardTimer/Data/Events/F_BumperEvent` _output)) (`self.currentTime`)))
      (`self.Activate Bumper Event` _output)
      (`/Engine/EditorBlueprintResources/StandardMacros.IncrementInt` (`self.currentBumperEvent`)))))

(fn `AdvanceMeteorPatternEvents`
  (bind _meteorpatternschedule (break `/Game/Systems/Blueprints/GM1/Hazards/HazardTimer/Data/F_HazardSchedule` (`self.activeSchedule`)))
  (bind _returnvalue (`KismetArrayLibrary.Array_Length` _meteorpatternschedule))
  (bind _returnvalue_2 (< (`self.currentMeteorPatternEvent`) _returnvalue))
  (bind _output (`|GetArrayItem` _meteorpatternschedule (`KismetMathLibrary.Clamp` (`self.currentMeteorPatternEvent`) 0 (- _returnvalue 1))))
  (if _returnvalue_2
    ;[0 0 0 0.5] While loop ensures that multiple events scheduled for the same time will trigger on the same frame. Take care not to start too many (>10) events at the same time, though.
    (while (and _returnvalue_2 (<= (`.EventTime_2_7D465B0C493681F68D63EB8966E30630` (break `/Game/Systems/Blueprints/GM1/Hazards/HazardTimer/Data/Events/F_MeteorPatternEvent` _output)) (`self.currentTime`)))
      (`self.Activate Meteor Pattern Event` _output)
      (`/Engine/EditorBlueprintResources/StandardMacros.IncrementInt` (`self.currentMeteorPatternEvent`)))))

(fn `AdvanceMeteorShowerEvents`
  (bind (_meteorpatternschedule _meteorshowerschedule) (break `/Game/Systems/Blueprints/GM1/Hazards/HazardTimer/Data/F_HazardSchedule` (`self.activeSchedule`)))
  (bind _returnvalue (`KismetArrayLibrary.Array_Length` _meteorshowerschedule))
  (bind _returnvalue_2 (< (`self.currentMeteorShowerEvent`) _returnvalue))
  (bind _output (`|GetArrayItem` _meteorshowerschedule (`KismetMathLibrary.Clamp` (`self.currentMeteorShowerEvent`) 0 (- _returnvalue 1))))
  (if _returnvalue_2
    ;[0 0 0 0.5] While loop ensures that multiple events scheduled for the same time will trigger on the same frame. Take care not to start too many (>10) events at the same time, though.
    (while (and _returnvalue_2 (<= (`.EventTime_2_54A3822C4DBAC6D0503955B89C2C4FE1` (break `/Game/Systems/Blueprints/GM1/Hazards/HazardTimer/Data/Events/F_MeteorShowerEvent` _output)) (`self.currentTime`)))
      (`self.Activate Meteor Shower Event` _output)
      (`/Engine/EditorBlueprintResources/StandardMacros.IncrementInt` (`self.currentMeteorShowerEvent`)))))

(fn `AdvanceWallEvents`
  (bind (_meteorpatternschedule _meteorshowerschedule _bumperschedule _arenahazardschedule _wallschedule) (break `/Game/Systems/Blueprints/GM1/Hazards/HazardTimer/Data/F_HazardSchedule` (`self.activeSchedule`)))
  (bind _returnvalue (`KismetArrayLibrary.Array_Length` _wallschedule))
  (bind _returnvalue_2 (< (`self.currentWallEvent`) _returnvalue))
  (bind _output (`|GetArrayItem` _wallschedule (`KismetMathLibrary.Clamp` (`self.currentWallEvent`) 0 (- _returnvalue 1))))
  (if _returnvalue_2
    ;[0 0 0 0.5] While loop ensures that multiple events scheduled for the same time will trigger on the same frame. Take care not to start too many (>10) events at the same time, though.
    (while (and _returnvalue_2 (<= (`.EventTime_13_EACB8D8A4080DF36CC532194BD113B16` (break `/Game/Systems/Blueprints/GM1/Hazards/HazardTimer/Data/Events/F_WallHazardEvent` _output)) (`self.currentTime`)))
      (`self.Activate Wall Event` _output)
      (`/Engine/EditorBlueprintResources/StandardMacros.IncrementInt` (`self.currentWallEvent`)))))

(fn `Get Valid Meteor Spawner`
  (returns (spawner :type "/Game/Systems/Blueprints/GM1/Hazards/Meteors/BP_GM1_MeteorSpawner Object Reference"))
  ;[1 0.7481 0 0.5] Note that this may return an unintended spawner. As such, be careful with this function by avoiding actions that may overwrite the output spawner's settings.
  (bind _returnvalue (`GameplayStatics.GetActorOfClass` "/Game/Systems/Blueprints/GM1/Hazards/Meteors/BP_GM1_MeteorSpawner.BP_GM1_MeteorSpawner_C"))
  (`/Engine/EditorBlueprintResources/StandardMacros.IsValid` _returnvalue
    (:`Is Valid`
      (return _returnvalue))
    (:`Is Not Valid`
      (bind _returnvalue_2 (`|SpawnActorFromClass` "/Game/Systems/Blueprints/GM1/Hazards/Meteors/BP_GM1_MeteorSpawner.BP_GM1_MeteorSpawner_C" (`KismetMathLibrary.MakeTransform` (0.0 0.0 25.0)) "Undefined" "MultiplyWithRoot" null "/Game/Systems/Blueprints/GM1/Hazards/Meteors/Data/DA_MeteorSpawner-CodeOnlySpawner.DA_MeteorSpawner-CodeOnlySpawner" null))
      (return _returnvalue_2))))

(fn `PauseSchedule`
  (set `self.IsPlaying` false))

(fn `SelectSchedule`
  (returns (Schedule :type "/Game/Systems/Blueprints/GM1/Hazards/HazardTimer/Data/F_HazardSchedule Structure"))
  (locals (index :type Integer))
  (bind (_userandomschedule _usescheduleatindex _schedules) (break `/Game/Systems/Blueprints/GM1/Hazards/HazardTimer/Data/F_ScheduleSelector` (`self.Schedule Data`)))
  (if _userandomschedule
    (set `local.index` (`KismetMathLibrary.RandomIntegerInRange` 0 (- (`KismetArrayLibrary.Array_Length` _schedules) 1)))
    (else
      (set `local.index` _usescheduleatindex)))
  (bind _output_get (set `self.activeSchedule` (`|GetArrayItem` _schedules (`local.index`))))
  (return _output_get))

(fn `SortAllSchedules`
  (locals (sortedSchedules :type "Array of /Game/Systems/Blueprints/GM1/Hazards/HazardTimer/Data/F_HazardSchedule Structure"))
  (bind _schedule_data (`self.Schedule Data`))
  (for _array_element (`.Schedules_10_F9155F24402F5EC8024A07A304801748` (break `/Game/Systems/Blueprints/GM1/Hazards/HazardTimer/Data/F_ScheduleSelector` _schedule_data))
    (bind (_meteorpatternschedule _meteorshowerschedule _bumperschedule _arenahazardschedule _wallschedule) (break `/Game/Systems/Blueprints/GM1/Hazards/HazardTimer/Data/F_HazardSchedule` _array_element))
    ;[0 0 0 0.5] We can't directly modify each array of the struct. Instead, we have to get a sorted copy of the array and then deliberately overwrite the original. We have to do the same with the array of schedules in the overall struct.
    ; In summary: why the fuck are structs so damn hard to work with?
    (bind _sortedschedule (`self.SortMeteorPatternSchedule` _meteorpatternschedule))
    (bind _sortedschedule_2 (`self.SortMeteorShowerSchedule` _meteorshowerschedule))
    (bind _sortedschedule_3 (`self.SortBumperSchedule` _bumperschedule))
    (bind _sortedschedule_4 (`self.SortArenaHazardSchedule` _arenahazardschedule))
    (bind _sortedschedule_5 (`self.SortWallSchedule` _wallschedule))
    (bind _structout (setmembers `/Game/Systems/Blueprints/GM1/Hazards/HazardTimer/Data/F_HazardSchedule` :`StructRef` _array_element :`Meteor Pattern Schedule` _sortedschedule :`Meteor Shower Schedule` _sortedschedule_2 :`Bumper Schedule` _sortedschedule_3 :`Arena Hazard Schedule` _sortedschedule_4 :`Wall Schedule` _sortedschedule_5))
    (`KismetArrayLibrary.Array_AddUnique` (`local.sortedSchedules`) _structout))
  (setmembers `/Game/Systems/Blueprints/GM1/Hazards/HazardTimer/Data/F_ScheduleSelector` :`StructRef` _schedule_data :`Schedules` (`local.sortedSchedules`)))

(fn `SortArenaHazardSchedule`
  (params (schedule :type "Array of /Game/Systems/Blueprints/GM1/Hazards/HazardTimer/Data/Events/F_ArenaHazardEvent Structure"))
  (returns (sortedSchedule :type "Array of /Game/Systems/Blueprints/GM1/Hazards/HazardTimer/Data/Events/F_ArenaHazardEvent Structure"))
  (for (_array_element _array_index) schedule
    (for _index (range _array_index (`KismetArrayLibrary.Array_Length` schedule))
      (if (< (`.EventTime_26_97FD4C2C4CD31F34555A7AA230F32490` (break `/Game/Systems/Blueprints/GM1/Hazards/HazardTimer/Data/Events/F_ArenaHazardEvent` (`|GetArrayItem` schedule _index))) (`.EventTime_26_97FD4C2C4CD31F34555A7AA230F32490` (break `/Game/Systems/Blueprints/GM1/Hazards/HazardTimer/Data/Events/F_ArenaHazardEvent` _array_element)))
        (`KismetArrayLibrary.Array_Swap` schedule _index _array_index))))
  (return (`local.schedule`)))

(fn `SortBumperSchedule`
  (params (schedule :type "Array of /Game/Systems/Blueprints/GM1/Hazards/HazardTimer/Data/Events/F_BumperEvent Structure"))
  (returns (sortedSchedule :type "Array of /Game/Systems/Blueprints/GM1/Hazards/HazardTimer/Data/Events/F_BumperEvent Structure"))
  (for (_array_element _array_index) schedule
    (for _index (range _array_index (`KismetArrayLibrary.Array_Length` schedule))
      (if (< (`.EventTime_10_4C73EC23445F080D0654368106218ACC` (break `/Game/Systems/Blueprints/GM1/Hazards/HazardTimer/Data/Events/F_BumperEvent` (`|GetArrayItem` schedule _index))) (`.EventTime_10_4C73EC23445F080D0654368106218ACC` (break `/Game/Systems/Blueprints/GM1/Hazards/HazardTimer/Data/Events/F_BumperEvent` _array_element)))
        (`KismetArrayLibrary.Array_Swap` schedule _index _array_index))))
  (return (`local.schedule`)))

(fn `SortMeteorPatternSchedule`
  (params (schedule :type "Array of /Game/Systems/Blueprints/GM1/Hazards/HazardTimer/Data/Events/F_MeteorPatternEvent Structure"))
  (returns (sortedSchedule :type "Array of /Game/Systems/Blueprints/GM1/Hazards/HazardTimer/Data/Events/F_MeteorPatternEvent Structure"))
  (for (_array_element _array_index) schedule
    (for _index (range _array_index (`KismetArrayLibrary.Array_Length` schedule))
      (if (< (`.EventTime_2_7D465B0C493681F68D63EB8966E30630` (break `/Game/Systems/Blueprints/GM1/Hazards/HazardTimer/Data/Events/F_MeteorPatternEvent` (`|GetArrayItem` schedule _index))) (`.EventTime_2_7D465B0C493681F68D63EB8966E30630` (break `/Game/Systems/Blueprints/GM1/Hazards/HazardTimer/Data/Events/F_MeteorPatternEvent` _array_element)))
        (`KismetArrayLibrary.Array_Swap` schedule _index _array_index))))
  (return (`local.schedule`)))

(fn `SortMeteorShowerSchedule`
  (params (schedule :type "Array of /Game/Systems/Blueprints/GM1/Hazards/HazardTimer/Data/Events/F_MeteorShowerEvent Structure"))
  (returns (sortedSchedule :type "Array of /Game/Systems/Blueprints/GM1/Hazards/HazardTimer/Data/Events/F_MeteorShowerEvent Structure"))
  (for (_array_element _array_index) schedule
    (for _index (range _array_index (`KismetArrayLibrary.Array_Length` schedule))
      (if (< (`.EventTime_2_54A3822C4DBAC6D0503955B89C2C4FE1` (break `/Game/Systems/Blueprints/GM1/Hazards/HazardTimer/Data/Events/F_MeteorShowerEvent` (`|GetArrayItem` schedule _index))) (`.EventTime_2_54A3822C4DBAC6D0503955B89C2C4FE1` (break `/Game/Systems/Blueprints/GM1/Hazards/HazardTimer/Data/Events/F_MeteorShowerEvent` _array_element)))
        (`KismetArrayLibrary.Array_Swap` schedule _index _array_index))))
  (return (`local.schedule`)))

(fn `SortWallSchedule`
  (params (schedule :type "Array of /Game/Systems/Blueprints/GM1/Hazards/HazardTimer/Data/Events/F_WallHazardEvent Structure"))
  (returns (sortedSchedule :type "Array of /Game/Systems/Blueprints/GM1/Hazards/HazardTimer/Data/Events/F_WallHazardEvent Structure"))
  (for (_array_element _array_index) schedule
    (for _index (range _array_index (`KismetArrayLibrary.Array_Length` schedule))
      (if (< (`.EventTime_13_EACB8D8A4080DF36CC532194BD113B16` (break `/Game/Systems/Blueprints/GM1/Hazards/HazardTimer/Data/Events/F_WallHazardEvent` (`|GetArrayItem` schedule _index))) (`.EventTime_13_EACB8D8A4080DF36CC532194BD113B16` (break `/Game/Systems/Blueprints/GM1/Hazards/HazardTimer/Data/Events/F_WallHazardEvent` _array_element)))
        (`KismetArrayLibrary.Array_Swap` schedule _index _array_index))))
  (return (`local.schedule`)))

(fn `StartSchedule`
  (`self.SortAllSchedules`)
  (set `self.IsPlaying` true))

(fn `UserConstructionScript`
  (`self.SelectSchedule`))