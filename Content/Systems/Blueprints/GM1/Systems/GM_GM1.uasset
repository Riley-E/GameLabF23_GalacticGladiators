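; GM_GM1 is the game mode for GM1, a timed local multiplayer crown minigame.
; It spawns connected players at start points, then runs a skippable intro cutscene and pregame countdown before starting the shared camera, hazard schedule and HUD.
; It tracks scores and announces new leaders through the FX manager.
; When time expires, it saves scores to the game instance and opens mid-game or final results, depending on tournament progress.
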(event `self.ReceiveBeginPlay`
  (`self.DoSetupGame`)
  (`/Game/Systems/Blueprints/BP_FXEventManager.GM1_IntroCutscene` (`self.FXManager`))
  ;[1 1 1] Forcing the UIIntroCutscene Sound Cue to play
  (bind _asgi_core_game_instance (cast `/Game/Core/Programming/Prototypes/GameData/GI_CORE_GameInstance` (`GameplayStatics.GetGameInstance`)))
  (bind _sound_cue (`/Game/Systems/Blueprints/GM1/Audio/BP_GM1_AudioAtlas.Get Sound Cue` (`/Game/Core/Programming/Prototypes/GameData/GI_CORE_GameInstance.SFXGM1AudioAtlas` _asgi_core_game_instance) "NewEnumerator48" false))
  (`GameplayStatics.PlaySound2D` _sound_cue 1.0 1.0 0.0 null null)
  (`self.IntroAnim`)
  (bind _returnvalue (`|CreateWidget` "/Game/Core/Programming/Prototypes/Test_Sai/WBP_CutsceneSkip.WBP_CutsceneSkip_C"))
  (`UserWidget.AddToViewport` _returnvalue 0)
  (add `MovieSceneSequencePlayer.OnStop` (`self.Sequence Player`) (delegate `StartPregameTimer`)))

(event `StartPregameTimer`
  (`Widget.RemoveFromParent` (stale `self.ReceiveBeginPlay` _returnvalue))
  (bind _returnvalue (`|CreateWidget` "/Game/Core/Programming/Prototypes/Test_Ryan/Widgets/WBP_Core_PregameCountdown.WBP_Core_PregameCountdown_C" null (`KismetMathLibrary.FTrunc` (`/Game/Systems/Blueprints/GM1/Gameplay/Data/PDA_Gameplay.Pregame Countdown Length` (`self.GameplayData`)))))
  (add `/Game/Core/Programming/Prototypes/Test_Ryan/Widgets/WBP_Core_PregameCountdown.OnTimerEnd` _returnvalue (delegate `Begin Round`))
  (`UserWidget.AddToViewport` _returnvalue 0))

(event `Begin Round`
  (`self.StartGame`)
  (for _array_element (`self.Players`)
    (`/Game/Systems/Blueprints/GM1/Player/Blueprints/BP_Player_GM1.Start Game Round` _array_element)))

(event `self.K2_OnRestartPlayer`
  (params (NewPlayer :type "Controller Object Reference"))
  (`parent.K2_OnRestartPlayer` NewPlayer))

(event `self.HandleStartingNewPlayer`
  (params (NewPlayer :type "PlayerController Object Reference"))
  ;[1 1 1] Possible Work Around
  (`parent.HandleStartingNewPlayer` NewPlayer)
  (`EnhancedInputSubsystemInterface.AddMappingContext` (pcsubsystem `EnhancedInputLocalPlayerSubsystem` NewPlayer) "/Game/Systems/Blueprints/GM1/Player/Input/IMC_GM1.IMC_GM1" 0 (struct)))

(event `IntroAnim`
  ;[0.1326 1 0] Intro Animation Cutscene
  (`/Game/Systems/Blueprints/BP_FXEventManager.GM1_IntroCutscene` (`self.FXManager`))
  (set `self.PlayingCutscene` true)
  (bind _returnvalue (`GameplayStatics.GetActorOfClass` "/Script/LevelSequence.LevelSequenceActor"))
  (set `self.Sequence Player` (`LevelSequenceActor.SequencePlayer` _returnvalue))
  (`MovieSceneSequencePlayer.Play` (`self.Sequence Player`))
  (set `self.CutsceneDuration` (`TimeManagementBlueprintLibrary.Conv_QualifiedFrameTimeToSeconds` (`MovieSceneSequencePlayer.GetDuration` (`self.Sequence Player`))))
  (`self.OnCutsceneEnd` :!label _label))

(event `SkipCutscene`
  ;[0.1326 1 0] Intro Animation Cutscene
  (if (`MovieSceneSequencePlayer.IsPlaying` (`self.Sequence Player`))
    (`MovieSceneSequencePlayer.GoToEndAndStop` (`self.Sequence Player`))
    (goto _label)))

(event `OnCutsceneEnd`
  ;[0.1326 1 0] Intro Animation Cutscene
  (if (`self.PlayingCutscene`)
    (set `self.PlayingCutscene` false)
    (`GameplayStatics.GetActorOfClass` "/Script/Engine.CameraActor")))

(event `TenSecondsRemain`
  (`/Game/Systems/Blueprints/BP_FXEventManager.GM1_TenSecondsLeft` (`self.FXManager`))
  (`KismetSystemLibrary.Delay` 5.0)
  (`/Game/Systems/Blueprints/BP_FXEventManager.GM1_Countdown` (`self.FXManager`) 0.0 0.0)
  (`KismetSystemLibrary.Delay` 1.0))

(event `AnnounceWinner`
  (`/Game/Systems/Blueprints/BP_FXEventManager.GM1_GameEnd` (`self.FXManager`))
  (`self.GameEnded`)
  (`KismetSystemLibrary.Delay` 7.0)
  (`self.GoToNextLevel`))

(fn `AdjustPlayerScore`
  (params (player :type "/Game/Systems/Blueprints/GM1/Player/Blueprints/BP_Player_GM1 Object Reference") (amount :type Integer))
  (bind _index (`/Game/Systems/Blueprints/GM1/Player/Blueprints/BP_Player_GM1.Index` player))
  (`BlueprintMapLibrary.Map_Add` (`self.PlayerScores`) _index (+ (`BlueprintMapLibrary.Map_Find` (`self.PlayerScores`) _index) (`local.amount`)))
  (`self.CalculateCurrentWinner`)
  (`/Game/Systems/Widgets/GM1/WBP_GM1_CrownMode.OnScoreChange` (`self.HUDWidget`) (`/Game/Systems/Blueprints/GM1/Player/Blueprints/BP_Player_GM1.Index` player)))

(fn `CalculateCurrentWinner`
  (returns (player :type Integer) (score :type Integer))
  (locals (maxScore :type Integer :default -1) (idOfMax :type Integer :default -1))
  (bind _keys (`BlueprintMapLibrary.Map_Keys` (`self.PlayerScores`)))
  (for _array_element _keys
    (bind _value (`BlueprintMapLibrary.Map_Find` (`self.PlayerScores`) _array_element))
    (if (> _value (`local.maxScore`))
      (set `local.maxScore` _value)
      (set `local.idOfMax` _array_element)))
  (if (!= (`self.currentWinnerIndex`) (`local.idOfMax`))
    (set `self.currentWinnerIndex` (`local.idOfMax`))
    (bind _asgm_gm1 (cast `/Game/Systems/Blueprints/GM1/Systems/GM_GM1` (`GameplayStatics.GetGameMode`)))
    (`/Game/Systems/Blueprints/BP_FXEventManager.GM1_NewFirstPlace` (`/Game/Systems/Blueprints/GM1/Systems/GM_GM1.FXManager` _asgm_gm1) (`local.idOfMax`)))
  (return (`local.idOfMax`) (`local.maxScore`)))

(fn `DoSetupGame`
  (returns (Failed :type Boolean))
  (locals (ConnectedPlayers :type "Array of /Game/Core/Programming/Prototypes/GameData/BP_PlayerData Structure"))
  ;[0 0 0 0.5] Get Camera Ref
  (bind _outactors (`GameplayStatics.GetAllActorsOfClass` "/Game/Systems/Blueprints/GM1/Camera/CM_GM1.CM_GM1_C"))
  (set `self.CameraRef` (`|GetArrayItem` _outactors))
  ;[0 0 0 0.5] Get FXManager ref
  (bind _returnvalue (`GameplayStatics.GetActorOfClass` "/Game/Systems/Blueprints/BP_FXEventManager.BP_FXEventManager_C"))
  (set `self.FXManager` _returnvalue)
  (`self.GetPlayerStartPoints`)
  ;[0 0 0 0.5] Game Instance
  (bind _asgi_core_game_instance (cast `/Game/Core/Programming/Prototypes/GameData/GI_CORE_GameInstance` (`GameplayStatics.GetGameInstance`)))
  (bind _output_get (set `self.Game Instance` _asgi_core_game_instance))
  (for (_ _array_index) (`/Game/Core/Programming/Prototypes/GameData/GI_CORE_GameInstance.PlayerData` _output_get)
    (bind _connected (`/Game/Core/Programming/Prototypes/GameData/GI_CORE_GameInstance.GetPlayerConnected` (`self.Game Instance`) _array_index))
    (if _connected
      (`self.SpawnPlayer` _array_index (`|GetArrayItem` (`self.PlayerStarts`) _array_index)))
    (bind _returnvalue_2 (`GameplayStatics.GetPlayerController` _array_index))
    (`/Engine/EditorBlueprintResources/StandardMacros.IsValid` _returnvalue_2
      (:`Is Valid`
        (`PlayerController.SetViewTargetWithBlend` _returnvalue_2 (`self.CameraRef`) 0.0 "VTBlend_Linear" 0.0 false))))
  (return false))

(fn `End Game`
  (set `self.isInGame` false)
  (bind _asgi_core_game_instance (cast `/Game/Core/Programming/Prototypes/GameData/GI_CORE_GameInstance` (`GameplayStatics.GetGameInstance`)))
  (`/Game/Core/Programming/Prototypes/GameData/GI_CORE_GameInstance.Play Music` _asgi_core_game_instance "NewEnumerator3" 0.0)
  (`KismetSystemLibrary.PrintString` "GameEnded")
  (`self.SetPlayerScores`)
  (`self.AnnounceWinner`))

(fn `FreePlayerCast`
  (returns (Result :type "/Game/Systems/Blueprints/GM1/Player/Blueprints/BP_Player_GM1 Object Reference"))
  (return null))

(fn `GetActivePlayers`
  (returns (Players :type "Array of /Game/Systems/Blueprints/GM1/Player/Blueprints/BP_Player_GM1 Object Reference") (Count :type Integer))
  (bind _players (`self.Players`))
  (return _players (`KismetArrayLibrary.Array_Length` _players)))

(fn `GetCurrentWinnerInfo`
  (returns (playerID :type Integer) (score :type Integer))
  (bind _currentwinnerindex (`self.currentWinnerIndex`))
  (return _currentwinnerindex (`BlueprintMapLibrary.Map_Find` (`self.PlayerScores`) _currentwinnerindex)))

(fn `GetIsInGame`
  (returns (IsInGame :type Boolean))
  (return (`self.isInGame`)))

(fn `GetPlayerScore`
  (params (`Player Index` :type Integer))
  (returns (Score :type Integer))
  (locals (scr :type Integer))
  (bind (_value _returnvalue) (`BlueprintMapLibrary.Map_Find` (`self.PlayerScores`) `Player Index`))
  (if _returnvalue
    (set `local.scr` _value)
    (else
      (set `local.scr` 0)))
  (return (`local.scr`)))

(fn `GetPlayerStartPoints`
  (bind _outactors (`GameplayStatics.GetAllActorsOfClass` "/Game/Systems/Blueprints/GM1/Systems/BP_GM1_PlayerStart.BP_GM1_PlayerStart_C"))
  (set `self.PlayerStarts` _outactors))

(fn `GoToNextLevel`
  (`KismetSystemLibrary.PrintString` "GoToNextLevel" true true (struct :`R` 1.0 :`G` 0.617634 :`B` 0.12172 :`A` 1.0) 20.0)
  ;[1 0.5556 0.07462] For Tournament Mode, will go to GM2 if TournamentMode is enabled (Sai)
  (bind _canmovetonextlevel (`/Game/Core/Programming/Prototypes/GameData/GI_CORE_GameInstance.CanGoToNextTournamentLevel` (`self.Game Instance`)))
  (if _canmovetonextlevel
    (set `/Game/Core/Programming/Prototypes/GameData/GI_CORE_GameInstance.LastPlayedGameMode` "NewEnumerator0" (`self.Game Instance`))
    (`GameplayStatics.OpenLevelBySoftObjectPtr` "/Game/Core/Programming/Prototypes/Test_Kellyn/Maps/MidGameResultsScreen.MidGameResultsScreen")
    (else
      (`GameplayStatics.OpenLevelBySoftObjectPtr` "/Game/Core/Programming/Prototypes/Test_Kellyn/Maps/FinalResultsScreen.FinalResultsScreen"))))

(fn `RemovePlayer`
  (params (PlayerToRemove :type "/Game/Systems/Blueprints/GM1/Player/Blueprints/BP_Player_GM1 Object Reference"))
  (returns (Return :type Boolean))
  (`/Game/Systems/Blueprints/GM1/Camera/CM_GM1.Remove Tracked Target` (`self.CameraRef`) PlayerToRemove)
  (return false))

(fn `RemoveUnusedCameras`
  (bind _outactors (`GameplayStatics.GetAllActorsOfClass` "/Script/Engine.CameraActor"))
  (for _array_element _outactors
    (`self.K2_DestroyActor` _array_element)))

(fn `ResetGame`
  (returns (Return :type Boolean))
  (bind _result (`|FormatText` "starts {s} \nplayers {p}controllers {c}" (`KismetArrayLibrary.Array_Length` (`self.PlayerStarts`)) (`KismetArrayLibrary.Array_Length` (`self.Players`)) (`KismetArrayLibrary.Array_Length` (`self.PlayerControllers`))))
  (`/Engine/EditorBlueprintResources/StandardMacros.DoOnce` false
    (:`Completed`
      (`KismetSystemLibrary.PrintText` _result)
      (`self.RestartGame`)
      (`self.DoSetupGame`)
      (`KismetSystemLibrary.PrintText` _result)
      (return true))))

(fn `SetPlayerScores`
  (locals (GI :type "/Game/Core/Programming/Prototypes/GameData/GI_CORE_GameInstance Object Reference"))
  (bind _gi (`local.GI`))
  (bind _asgi_core_game_instance (cast `/Game/Core/Programming/Prototypes/GameData/GI_CORE_GameInstance` (`GameplayStatics.GetGameInstance`)))
  (set `local.GI` _asgi_core_game_instance)
  (for _array_element (`self.Players`)
    (bind _index (`/Game/Systems/Blueprints/GM1/Player/Blueprints/BP_Player_GM1.Index` _array_element))
    (bind _score (`self.GetPlayerScore` _index))
    (`/Game/Core/Programming/Prototypes/GameData/GI_CORE_GameInstance.AddPlayerScore` _gi _score _index)
    (`/Game/Core/Programming/Prototypes/GameData/GI_CORE_GameInstance.AddWins` _gi)))

(fn `ShouldReset`
  (params (ActorToReset :type "Actor Object Reference"))
  (returns (ReturnValue :type Boolean))
  (return false))

(fn `SpawnPlayer`
  (params (CurrentPlayerIndex :type Integer) (PlayerStart :type "/Game/Systems/Blueprints/GM1/Systems/BP_GM1_PlayerStart Object Reference"))
  (returns (Return :type Boolean))
  ;[0 0 0 0.5] Spawn Player Pawn and Possess
  (bind _returnvalue (`|SpawnActorFromClass` "/Game/Systems/Blueprints/GM1/Player/Blueprints/BP_Player_GM1.BP_Player_GM1_C" (`self.GetTransform` PlayerStart) "Undefined" "MultiplyWithRoot" null CurrentPlayerIndex (`self.PregameTimer`) null))
  (`KismetArrayLibrary.Array_Add` (`self.Players`) _returnvalue)
  (`BlueprintMapLibrary.Map_Add` (`self.PlayerScores`) CurrentPlayerIndex)
  (`Controller.Possess` (`GameplayStatics.GetPlayerController` CurrentPlayerIndex) _returnvalue)
  (return true))

(fn `StartGame`
  (returns (Return :type Boolean))
  (bind _returnvalue (`KismetMathLibrary.Conv_IntToDouble` (`/Game/Systems/Blueprints/GM1/Gameplay/Data/PDA_Gameplay.gameDurationInSeconds` (`self.GameplayData`))))
  (if (>= (`KismetArrayLibrary.Array_Length` (`self.Players`)) (`self.MinPlayers`))
    (set `self.isInGame` true)
    (`/Game/Systems/Blueprints/GM1/Camera/CM_GM1.GameStarted` (`self.CameraRef`) (`self.Players`))
    (bind _returnvalue_2 (`GameplayStatics.GetActorOfClass` "/Game/Systems/Blueprints/GM1/Hazards/HazardTimer/BP_HazardTimer.BP_HazardTimer_C"))
    (`/Game/Systems/Blueprints/GM1/Hazards/HazardTimer/BP_HazardTimer.StartSchedule` _returnvalue_2)
    (bind _returnvalue_3 (`GameplayStatics.GetActorOfClass` "/Game/Systems/Blueprints/GM1/BP_Crown.BP_Crown_C"))
    ;[0.1317 0.5622 1] Has dependencies
    (bind _returnvalue_4 (`|CreateWidget` "/Game/Systems/Widgets/GM1/WBP_GM1_CrownMode.WBP_GM1_CrownMode_C" null _returnvalue_3))
    (set `self.HUDWidget` _returnvalue_4)
    (`UserWidget.AddToViewport` _returnvalue_4 0) ; Adds old UI and timer widget
    (for _array_element (`self.Players`)
      (add `/Game/Systems/Blueprints/GM1/Player/Blueprints/BP_Player_GM1.OnAdjustPlayerScore` _array_element (`|CreateDelegate` :!event `AdjustPlayerScore`))
      ;[0.1317 0.5622 1] Creates new HUD version
      (bind _returnvalue_5 (`|CreateWidget` "/Game/Core/Programming/Prototypes/UI_Team/UI_Widgets/WBP_HUD_PlayerHUD.WBP_HUD_PlayerHUD_C"))
      (bind _output_get (set `self.HUDWidgetNew` _returnvalue_5))
      (`UserWidget.AddToViewport` _output_get 0)
      (`/Game/Core/Programming/Prototypes/UI_Team/UI_Widgets/WBP_HUD_PlayerHUD.InitializeHUD` _output_get self))
    (`KismetSystemLibrary.K2_SetTimer` null "TenSecondsRemain" (- _returnvalue 10.0))
    (`KismetSystemLibrary.K2_SetTimer` null "End Game" _returnvalue)
    (`KismetSystemLibrary.PrintString` "GameStarted")
    (`/Game/Core/Programming/Prototypes/GameData/GI_CORE_GameInstance.IncrementNumGamesPlayed` (`self.Game Instance`))
    (`self.GameStarted`)
    (`/Game/Systems/Blueprints/BP_FXEventManager.GM1_GameStart` (`self.FXManager`))
    (return false)))

(fn `UserConstructionScript`)