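; Crown pickup for the GM1 mode that players carry to earn score on a looping timer.
; An uncontrolled crown goes to an eligible overlapping player and follows their head socket with a velocity-based offset.
; Tick also spins and bobs it, or moves it to a random spawn point around its origin until it lands.
; Reset plays a respawn timeline before reselecting a spot, while camera tracking, decal and FX follow state changes.
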(event `self.ReceiveBeginPlay`
  (bind _asgm_gm1 (cast `/Game/Systems/Blueprints/GM1/Systems/GM_GM1` (`GameplayStatics.GetGameMode`)))
  (add `/Game/Systems/Blueprints/GM1/Systems/GM_GM1.GameStarted` _asgm_gm1 (`|CreateDelegate` :!event `SelectStartPosition`)))

(event `self.ReceiveActorBeginOverlap`
  (params (OtherActor :type "Actor Object Reference"))
  ;[0 0 0] If a player is touching and the crowned is not currently controlled, give control to that player
  (`/Engine/EditorBlueprintResources/StandardMacros.IsValid` (`self.Controlling Player`)
    (:`Is Not Valid`
      (bind _asbp_player_gm1 (cast `/Game/Systems/Blueprints/GM1/Player/Blueprints/BP_Player_GM1` OtherActor))
      (if (`/Game/Systems/Blueprints/GM1/Player/Blueprints/BP_Player_GM1.bCanHaveCrown` _asbp_player_gm1)
        (`/Game/Systems/Blueprints/GM1/Player/Blueprints/BP_Player_GM1.GiveCrown` _asbp_player_gm1 self)
        (bind _asgm_gm1 (cast `/Game/Systems/Blueprints/GM1/Systems/GM_GM1` (`GameplayStatics.GetGameMode`)))
        (`/Game/Systems/Blueprints/BP_FXEventManager.GM1_CrownPickedUp` (`/Game/Systems/Blueprints/GM1/Systems/GM_GM1.FXManager` _asgm_gm1) self _asbp_player_gm1)))))

(event `self.ReceiveTick`
  (params (DeltaSeconds :type "Float (single-precision)"))
  (`self.LerpToPosition`)
  (`self.Bob and Spin`))

(event `Reset`
  (bind (_returnvalue_x _returnvalue_y _returnvalue_z) (`KismetMathLibrary.BreakVector` (`self.K2_GetActorLocation`)))
  (bind (_resetlocation_x _resetlocation_y _resetlocation_z) (`KismetMathLibrary.BreakVector` (`self.resetLocation`)))
  (bind _respawn_timeline (`self.Respawn Timeline`))
  (bind _returnvalue (/ (`TimelineComponent.GetPlaybackPosition` _respawn_timeline) (`TimelineComponent.GetTimelineLength` _respawn_timeline)))
  (`SceneComponent.SetVisibility` (`self.Decal`) false false)
  (bind _returnvalue_2 (`GameplayStatics.GetActorOfClass` "/Game/Systems/Blueprints/GM1/Camera/CM_GM1.CM_GM1_C"))
  (`/Game/Systems/Blueprints/GM1/Camera/CM_GM1.Remove Tracked Target` _returnvalue_2 self)
  (set `self.bCrownActive` false)
  (set `self.bReachedSpawn` false)
  (bind (_direction _height_scalar) (`Timeline|Respawn Timeline` :!via `PlayFromStart`)
    (:`Update`
      (`self.K2_SetActorLocation` (+ (`KismetMathLibrary.VLerp` (`KismetMathLibrary.MakeVector` _returnvalue_x _returnvalue_y) (`KismetMathLibrary.MakeVector` _resetlocation_x _resetlocation_y) _returnvalue) (`KismetMathLibrary.MakeVector` 0.0 0.0 (`KismetMathLibrary.Lerp` _returnvalue_z (+ _resetlocation_z (* _height_scalar 4500.0)) _returnvalue)))))
    (:`Finished`
      (`self.SelectStartPosition`))))

(fn `AwardScore`
  (`/Game/Systems/Blueprints/GM1/Player/Blueprints/BP_Player_GM1.EarnCrownScore` (`self.Controlling Player`) (`/Game/Systems/Blueprints/GM1/Data/PDA_Crown.baseScoreValue` (`self.CrownData`)))
  ;[0 0 0] Flash the crown material. Should be deprecated when a VFX asset has been created
  (`PrimitiveComponent.SetMaterial` (`self.Crown`) 1 "/Game/GameMode1/Art/Materials/Material_Instances/MI_Metal_Gold.MI_Metal_Gold")
  (`KismetSystemLibrary.K2_SetTimer` null "StopFlash" 0.1))

(fn `Bob and Spin`
  ;[0 0 0] Spin
  (`SceneComponent.K2_SetWorldRotation` (`self.Crown`) (`KismetMathLibrary.ComposeRotators` (`SceneComponent.K2_GetComponentRotation` (`self.Crown`)) (`KismetMathLibrary.MakeRotator` 0.0 0.0 (* (`GameplayStatics.GetWorldDeltaSeconds`) 135.0))) false false)
  ;[0 0 0] Bob if the crown is not traveling to its spawn point when the game begins or when a player falls off the edge
  (if (or (not (`self.bCrownActive`)) (`self.bReachedSpawn`))
    (`SceneComponent.K2_AddWorldOffset` (`self.Crown`) (`KismetMathLibrary.MakeVector` 0.0 0.0 (`KismetMathLibrary.DegSin` (* (`GameplayStatics.GetTimeSeconds`) 90.0))) false false)))

(fn `Clear Control`
  (params (addToCameraTracking :type Boolean))
  ;[0 0 0] Stop awarding the controlling player points
  (if (!= (`KismetSystemLibrary.K2_GetTimerRemainingTime` null "AwardScore") 0.0)
    (`KismetSystemLibrary.K2_ClearTimer` null "AwardScore"))
  (set `self.Controlling Player` null)
  ;[0 0 0] Stop following the previous player and display decal
  (`SceneComponent.SetVisibility` (`self.Decal`) true false)
  (`SceneComponent.K2_SetRelativeRotation` :`self` (`self.RootComponent`))
  ;[0 0 0] Add to camera tracking if necessary
  (if addToCameraTracking
    (bind _returnvalue (`GameplayStatics.GetActorOfClass` "/Game/Systems/Blueprints/GM1/Camera/CM_GM1.CM_GM1_C"))
    (`/Game/Systems/Blueprints/GM1/Camera/CM_GM1.Add Tracked Target` _returnvalue self)
    (`self.OnDrop`)))

(fn `LerpToPosition`
  (bind _returnvalue (`self.K2_GetActorLocation`))
  (bind _returnvalue_2 (`self.K2_GetActorLocation`))
  (bind _controlling_player (`self.Controlling Player`))
  (`/Engine/EditorBlueprintResources/StandardMacros.IsValid` (`self.Controlling Player`)
    (:`Is Valid`
      (`self.K2_SetActorLocation` (+ (`SceneComponent.GetSocketLocation` (`Character.Mesh` (`self.Controlling Player`)) "CrownSocket") (0.0 0.0 0.0)))
      ;[0 0 0] Ignore rotation caused by parent transform
      (`SceneComponent.K2_SetWorldRotation` :`self` (`self.RootComponent`))
      ;[0 0 0] Add a small offset to create a lagging follow effect
      (`self.K2_AddActorWorldOffset` (* (/ (`self.GetVelocity` _controlling_player) (`/Game/Systems/Blueprints/GM1/Player/Systems/Data/PDA_Player_GM1.BaseMovementSpeed` (`/Game/Systems/Blueprints/GM1/Player/Blueprints/BP_Player_GM1.PlayerData` _controlling_player))) (`/Game/Systems/Blueprints/GM1/Data/PDA_Crown.followLerpAlpha` (`self.CrownData`)))))
    (:`Is Not Valid`
      (if (`self.bReachedSpawn`)
        (`self.K2_SetActorLocation` (`KismetMathLibrary.VLerp` _returnvalue (`KismetMathLibrary.MakeVector` (.x _returnvalue) (.y _returnvalue) (`/Game/Systems/Blueprints/GM1/Data/PDA_Crown.defaultFloatHeight` (`self.CrownData`))) (`/Game/Systems/Blueprints/GM1/Data/PDA_Crown.followLerpAlpha` (`self.CrownData`))))
        (elif (`self.bCrownActive`)
          (`self.K2_SetActorLocation` (`KismetMathLibrary.VLerp` _returnvalue_2 (`KismetMathLibrary.MakeVector` (.x (`self.targetStart`)) (.y (`self.targetStart`)) (.z _returnvalue_2)) (`/Game/Systems/Blueprints/GM1/Data/PDA_Crown.followLerpAlpha` (`self.CrownData`))))
          ;[0 0 0] Fall toward the default float height
          (bind _sweephitresult (`self.K2_AddActorWorldOffset` (`KismetMathLibrary.MakeVector` 0.0 0.0 (* (`KismetMathLibrary.FClamp` (* (`/Game/Systems/Blueprints/GM1/Data/PDA_Crown.initialFallSpeed` (`self.CrownData`)) (`GameplayStatics.GetWorldDeltaSeconds`)) 0.0 (- (.z (`self.K2_GetActorLocation`)) (`/Game/Systems/Blueprints/GM1/Data/PDA_Crown.defaultFloatHeight` (`self.CrownData`)))) -1.0)) true))
          (bind (_bblockinghit _binitialoverlap) (`GameplayStatics.BreakHitResult` _sweephitresult))
          ;[0 0 0] If the crown is at the default float height and target position, marked spawn as reached
          (bind _output_get (set `self.bReachedSpawn` (or _bblockinghit _binitialoverlap (== (`self.K2_GetActorLocation`) (`KismetMathLibrary.MakeVector` (.x (`self.targetStart`)) (.y (`self.targetStart`)) (`/Game/Systems/Blueprints/GM1/Data/PDA_Crown.defaultFloatHeight` (`self.CrownData`))) :`ErrorTolerance` 0.01))))
          (if _output_get
            (bind _asgm_gm1 (cast `/Game/Systems/Blueprints/GM1/Systems/GM_GM1` (`GameplayStatics.GetGameMode`)))
            (`/Game/Systems/Blueprints/BP_FXEventManager.GM1_CrownSpawn` (`/Game/Systems/Blueprints/GM1/Systems/GM_GM1.FXManager` _asgm_gm1) self)))))))

(fn `PlayStealVFX`
  (bind _returnvalue (`self.K2_GetActorLocation`))
  (bind _asgi_core_game_instance (cast `/Game/Core/Programming/Prototypes/GameData/GI_CORE_GameInstance` (`GameplayStatics.GetGameInstance`)))
  (bind _gameinstancevariables (`/Game/Core/Programming/Prototypes/GameData/GI_CORE_GameInstance.GameInstanceVariables` _asgi_core_game_instance))
  (`NiagaraFunctionLibrary.SpawnSystemAtLocation` (`/Game/Core/Programming/Prototypes/Test_Sai/PDA_GameInstanceSettings.GM1_GenericCrownStealVFX` _gameinstancevariables) _returnvalue)
  (`GameplayStatics.PlaySoundAtLocation` (`/Game/Core/Programming/Prototypes/Test_Sai/PDA_GameInstanceSettings.GM1_GenericCrownStealSFX` _gameinstancevariables) _returnvalue (struct) 1.0 1.0 0.0 null null null null))

(fn `SelectStartPosition`
  (locals (arenaCenter :type "Vector Structure") (targetOffset :type "Vector Structure"))
  (bind _resetlocation (`self.resetLocation`))
  (bind (_lowerbound _upperbound) (break `FloatRange` (`/Game/Systems/Blueprints/GM1/Data/PDA_Crown.spawnRadiusRange` (`self.CrownData`))))
  ;[0 0 0] Add to camera tracking
  (bind _returnvalue (`GameplayStatics.GetActorOfClass` "/Game/Systems/Blueprints/GM1/Camera/CM_GM1.CM_GM1_C"))
  (`/Game/Systems/Blueprints/GM1/Camera/CM_GM1.Add Tracked Target` _returnvalue self)
  (`SceneComponent.SetVisibility` (`self.Decal`) true false)
  (`self.K2_SetActorLocation` _resetlocation)
  (set `self.targetStart` (+ _resetlocation (* (`KismetMathLibrary.Normal` (`KismetMathLibrary.MakeVector` (`KismetMathLibrary.RandomFloatInRange` -1.0 1.0) (`KismetMathLibrary.RandomFloatInRange` -1.0 1.0))) (`KismetMathLibrary.RandomFloatInRange` (`.Value` (break `FloatRangeBound` _lowerbound)) (`.Value` (break `FloatRangeBound` _upperbound))))))
  (set `self.bReachedSpawn` false)
  (set `self.bCrownActive` true)
  (bind _asgm_gm1 (cast `/Game/Systems/Blueprints/GM1/Systems/GM_GM1` (`GameplayStatics.GetGameMode`)))
  (`/Game/Systems/Blueprints/BP_FXEventManager.GM1_CrownPreSpawn` (`/Game/Systems/Blueprints/GM1/Systems/GM_GM1.FXManager` _asgm_gm1) self))

(fn `SetControl`
  (params (player :type "/Game/Systems/Blueprints/GM1/Player/Blueprints/BP_Player_GM1 Object Reference"))
  ;[0 0 0] Clear any previous control and set a new controlling player
  (`self.Clear Control` false)
  (set `self.Controlling Player` player)
  ;[0 0 0] Start awarding score to the new controlling player
  (`KismetSystemLibrary.K2_SetTimer` null "AwardScore" (`/Game/Systems/Blueprints/GM1/Data/PDA_Crown.baseScoreTime` (`self.CrownData`)) true)
  ;[0 0 0] Remove from camera tracking
  (bind _returnvalue (`GameplayStatics.GetActorOfClass` "/Game/Systems/Blueprints/GM1/Camera/CM_GM1.CM_GM1_C"))
  (`/Game/Systems/Blueprints/GM1/Camera/CM_GM1.Remove Tracked Target` _returnvalue self)
  (`SceneComponent.SetVisibility` (`self.Decal`) false false)
  (`self.OnPickup`))

(fn `StopFlash`
  (`PrimitiveComponent.SetMaterial` (`self.Crown`) 1 "/Game/GameMode1/Art/EnviormentAssets/Crown/MI_CrownEmissive.MI_CrownEmissive"))

(fn `UserConstructionScript`
  (`SphereComponent.SetSphereRadius` (`self.Collision`) (`/Game/Systems/Blueprints/GM1/Data/PDA_Crown.collisionRadius` (`self.CrownData`)) true)
  (set `self.resetLocation` (`self.K2_GetActorLocation`))
  (`SceneComponent.SetVisibility` (`self.Decal`) false false))