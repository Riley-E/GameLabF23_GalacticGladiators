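; BP_GM2_AudioAtlas is a lookup table for game mode 2 audio that maps event enum values to Sound Cues.
; GetSoundCue looks up the requested enum in the AudioClips map and returns its cue, or nothing when absent.
; Color-coded prints report hits and misses, but their local flag is set to false and the DebugMessage input is unused, so they stay silent.
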(fn `GetSoundCue`
  (params (Enum :type "/Game/Audio/E_GM2_AudioClips Enum" :default "NewEnumerator18") (`Debug Message` :type Boolean))
  (returns (SoundCue :type "SoundCue Object Reference"))
  (locals (dMess :type Boolean :default true) (RequestedEnum :type "/Game/Audio/E_GM2_AudioClips Enum" :default "NewEnumerator18"))
  (bind (_value _returnvalue) (`BlueprintMapLibrary.Map_Find` (`self.AudioClips`) (`local.RequestedEnum`)))
  (set `local.RequestedEnum` Enum)
  (set `local.dMess` false)
  (if _returnvalue
    (if (`local.dMess`)
      (`KismetSystemLibrary.PrintString` null (`KismetStringLibrary.Concat_StrStr` "[BP_GM2_AudioAtlas] Event {" (`|GetEnumeratorNameAsString` (`local.RequestedEnum`)) "} accessed the associated Sound Cue") true true (struct :`R` 0.252777 :`G` 1.0 :`B` 0.230999 :`A` 1.0)))
    (return _value)
    (else
      (if (`local.dMess`)
        (`KismetSystemLibrary.PrintString` null (`KismetStringLibrary.Concat_StrStr` "[BP_GM2_AudioAtlas] Event {" (`|GetEnumeratorNameAsString` (`local.RequestedEnum`)) "} has no associated Sound Cue") true true (struct :`R` 1.0 :`G` 0.155993 :`B` 0.175889 :`A` 1.0)))
      (return null))))