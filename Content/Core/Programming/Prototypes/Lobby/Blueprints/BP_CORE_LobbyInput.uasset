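; Per-player input handler for the lobby prototype, turning Enhanced Input actions into join, leave, character select, start and back-to-menu.
; BeginPlay caches the lobby widget, game mode and game instance.
; Join and leave update the connected state for its PlayerID in the game instance and notify the widget, which also receives selection changes.
; Join, leave or select cancels a running countdown instead; start asks the game mode to begin.
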(event `self.ReceiveBeginPlay`
  ;[0 0 0] Get Lobby Widget
  (bind _foundwidgets (`WidgetBlueprintLibrary.GetAllWidgetsOfClass` "/Game/Core/Programming/Prototypes/Lobby/Widgets/WBP_CORE_LobbyMenu.WBP_CORE_LobbyMenu_C"))
  (set `self.LobbyWidget` (`|GetArrayItem` _foundwidgets))
  ;[0 0 0] Set GameMode Variable
  (bind _asgm_core_lobby (cast `/Game/Core/Programming/Prototypes/Lobby/Blueprints/GM_CORE_Lobby` (`GameplayStatics.GetGameMode`)))
  (bind _output_get (set `self.GM` _asgm_core_lobby))
  (set `self.GI` (`/Game/Core/Programming/Prototypes/MultiplayerMenu/GM_Core_NoPlayerControllerInput.CurrentGameInstance` _output_get)))

(event `EnhancedInput|/Game/Core/Programming/Prototypes/Lobby/Input/IA_CORE_PrevSelect`
  (params (ActionValue :type Boolean) (ElapsedSeconds :type "Float (double-precision)") (TriggeredSeconds :type "Float (double-precision)") (InputAction :type "InputAction Object Reference" :default "/Game/Core/Programming/Prototypes/Lobby/Input/IA_CORE_PrevSelect.IA_CORE_PrevSelect"))
  (:`Started`
    (if (`/Game/Core/Programming/Prototypes/Lobby/Widgets/WBP_CORE_LobbyMenu.IsCountingDown` (`self.LobbyWidget`))
      (`/Game/Core/Programming/Prototypes/Lobby/Widgets/WBP_CORE_LobbyMenu.CancelGameCountdown` (`self.LobbyWidget`))
      (elif (`self.Joined`)
        (`self.SFX` "NewEnumerator0")
        ;[0 0 0] Trigger Character Change
        (`/Game/Core/Programming/Prototypes/Lobby/Widgets/WBP_CORE_LobbyMenu.SelectPreviousEvent` (`self.LobbyWidget`) (`self.PlayerID`))))))

(event `EnhancedInput|/Game/Core/Programming/Prototypes/Lobby/Input/IA_CORE_NextSelect`
  (params (ActionValue :type Boolean) (ElapsedSeconds :type "Float (double-precision)") (TriggeredSeconds :type "Float (double-precision)") (InputAction :type "InputAction Object Reference" :default "/Game/Core/Programming/Prototypes/Lobby/Input/IA_CORE_NextSelect.IA_CORE_NextSelect"))
  (:`Started`
    (if (`/Game/Core/Programming/Prototypes/Lobby/Widgets/WBP_CORE_LobbyMenu.IsCountingDown` (`self.LobbyWidget`))
      (`/Game/Core/Programming/Prototypes/Lobby/Widgets/WBP_CORE_LobbyMenu.CancelGameCountdown` (`self.LobbyWidget`))
      (elif (`self.Joined`)
        (`self.SFX` "NewEnumerator0")
        ;[0 0 0] Trigger Character Change
        (`/Game/Core/Programming/Prototypes/Lobby/Widgets/WBP_CORE_LobbyMenu.SelectNext_Event` (`self.LobbyWidget`) (`self.PlayerID`))))))

(event `EnhancedInput|/Game/Core/Programming/Prototypes/Lobby/Input/IA_CORE_Join`
  (params (ActionValue :type Boolean) (ElapsedSeconds :type "Float (double-precision)") (TriggeredSeconds :type "Float (double-precision)") (InputAction :type "InputAction Object Reference" :default "/Game/Core/Programming/Prototypes/Lobby/Input/IA_CORE_Join.IA_CORE_Join"))
  (bind _playerid (`self.PlayerID`))
  (:`Started`
    (if (`/Game/Core/Programming/Prototypes/Lobby/Widgets/WBP_CORE_LobbyMenu.IsCountingDown` (`self.LobbyWidget`))
      (`/Game/Core/Programming/Prototypes/Lobby/Widgets/WBP_CORE_LobbyMenu.CancelGameCountdown` (`self.LobbyWidget`))
      (else
        (set `self.Joined` true)
        (`self.SFX` "NewEnumerator8")
        ;[0 0 0] Player Joining Lobby (if GI says not joined)
        (bind _connected (`/Game/Core/Programming/Prototypes/GameData/GI_CORE_GameInstance.GetPlayerConnected` (`/Game/Core/Programming/Prototypes/MultiplayerMenu/GM_Core_NoPlayerControllerInput.CurrentGameInstance` (`self.GM`)) (`self.PlayerID`)))
        (if (not _connected)
          (`/Game/Core/Programming/Prototypes/GameData/GI_CORE_GameInstance.SetPlayerConnected` (`/Game/Core/Programming/Prototypes/MultiplayerMenu/GM_Core_NoPlayerControllerInput.CurrentGameInstance` (`self.GM`)) _playerid true)
          (`/Game/Core/Programming/Prototypes/Lobby/Widgets/WBP_CORE_LobbyMenu.PlayerJoined_Event` (`self.LobbyWidget`) (`self.PlayerID`))
          ;[1 1 1] Debug
          (`KismetSystemLibrary.PrintText` (`|FormatText` "BP: Player Joined {0}" _playerid)))))))

(event `EnhancedInput|/Game/Core/Programming/Prototypes/Lobby/Input/IA_CORE_Leave`
  (params (ActionValue :type Boolean) (ElapsedSeconds :type "Float (double-precision)") (TriggeredSeconds :type "Float (double-precision)") (InputAction :type "InputAction Object Reference" :default "/Game/Core/Programming/Prototypes/Lobby/Input/IA_CORE_Leave.IA_CORE_Leave"))
  (bind _playerid (`self.PlayerID`))
  (:`Started`
    (if (`/Game/Core/Programming/Prototypes/Lobby/Widgets/WBP_CORE_LobbyMenu.IsCountingDown` (`self.LobbyWidget`))
      (`/Game/Core/Programming/Prototypes/Lobby/Widgets/WBP_CORE_LobbyMenu.CancelGameCountdown` (`self.LobbyWidget`))
      (else
        (set `self.Joined` false)
        (`self.SFX` "NewEnumerator26")
        ;[0 0 0] Player Leaving Lobby
        (bind _connected (`/Game/Core/Programming/Prototypes/GameData/GI_CORE_GameInstance.GetPlayerConnected` (`/Game/Core/Programming/Prototypes/MultiplayerMenu/GM_Core_NoPlayerControllerInput.CurrentGameInstance` (`self.GM`)) (`self.PlayerID`)))
        (if _connected
          (`/Game/Core/Programming/Prototypes/Lobby/Widgets/WBP_CORE_LobbyMenu.PlayerLeft_Event` (`self.LobbyWidget`) (`self.PlayerID`))
          (`/Game/Core/Programming/Prototypes/GameData/GI_CORE_GameInstance.SetPlayerConnected` (`/Game/Core/Programming/Prototypes/MultiplayerMenu/GM_Core_NoPlayerControllerInput.CurrentGameInstance` (`self.GM`)) _playerid false)
          ;[1 1 1] Debug
          (`KismetSystemLibrary.PrintText` (`|FormatText` "BP: Player Left {0}" _playerid)))))))

(event `EnhancedInput|/Game/Core/Programming/Prototypes/Lobby/Input/IA_CORE_Start`
  (params (ActionValue :type Boolean) (ElapsedSeconds :type "Float (double-precision)") (TriggeredSeconds :type "Float (double-precision)") (InputAction :type "InputAction Object Reference" :default "/Game/Core/Programming/Prototypes/Lobby/Input/IA_CORE_Start.IA_CORE_Start"))
  (:`Started`
    (if (`self.Joined`)
      (`self.SFX` "NewEnumerator25")
      (`KismetSystemLibrary.Delay` 0.1)
      ;[0 0 0] Players Press Enter to Continue Game
      (`/Game/Core/Programming/Prototypes/Lobby/Blueprints/GM_CORE_Lobby.Try Game Start` (`self.GM`)))))

(event `EnhancedInput|/Game/Core/Programming/Prototypes/Lobby/Input/IA_Core_Back`
  (params (ActionValue :type Boolean) (ElapsedSeconds :type "Float (double-precision)") (TriggeredSeconds :type "Float (double-precision)") (InputAction :type "InputAction Object Reference" :default "/Game/Core/Programming/Prototypes/Lobby/Input/IA_Core_Back.IA_Core_Back"))
  (:`Started`
    (bind _cliplength (`self.SFX` "NewEnumerator2"))
    (`KismetSystemLibrary.Delay` _cliplength)
    (`GameplayStatics.OpenLevelBySoftObjectPtr` "/Game/Core/Programming/Prototypes/Test_Kellyn/Maps/MainMenu3D.MainMenu3D")))

(fn `UserConstructionScript`)