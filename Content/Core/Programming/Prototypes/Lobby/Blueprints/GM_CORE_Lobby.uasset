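; Lobby game mode that validates joined players and moves the game on to the next level.
; BeginPlay spawns input pawns and plays voice-over; TryGameStart requires a connected player (count > 0, despite "more than one" messaging) and unique models before starting the widget countdown.
; ContinueToLevel waits out lock-in VO, then opens a random pre-game screen in Tournament Mode, otherwise level select.
; Disconnected nodes hold older validation attempts.
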(event `self.ReceiveBeginPlay`
  (`self.SpawnInputPawns`)
  (bind _asgi_core_game_instance (cast `/Game/Core/Programming/Prototypes/GameData/GI_CORE_GameInstance` (`GameplayStatics.GetGameInstance`)))
  (bind _soundcue (`/Game/Audio/PDA_Core_AudioAtlas.GetSoundCue` (`/Game/Core/Programming/Prototypes/GameData/GI_CORE_GameInstance.VOLobbyAudioAtlas` _asgi_core_game_instance) "NewEnumerator30"))
  (`GameplayStatics.PlaySound2D` _soundcue 1.0 1.0 0.0 null null))

(event `Try Game Start`
  (bind _currentgameinstance (`self.CurrentGameInstance`))
  (bind _playerdata (`/Game/Core/Programming/Prototypes/GameData/GI_CORE_GameInstance.PlayerData` (`self.CurrentGameInstance`)))
  (`KismetSystemLibrary.PrintString` "GM: Try Game Start")
  ;[0 0 0] Check if more than one player has joined
  (set `self.PlayerCount` 0)
  (for _array_element (`/Game/Core/Programming/Prototypes/GameData/GI_CORE_GameInstance.PlayerData` (`self.CurrentGameInstance`))
    (if (`.PlayerConnected_5_AB8DC441490816CD933DC5B7A4919B1A` (break `/Game/Core/Programming/Prototypes/GameData/BP_PlayerData` _array_element))
      (`/Engine/EditorBlueprintResources/StandardMacros.IncrementInt` (`self.PlayerCount`))))
  (if (> (`self.PlayerCount`) 0)
    ;[0 0 0] Check players dont have the same models (not sure if this ever worked properly)
    (set `self.SameModel` false)
    (for (_array_element_2 _array_index) _playerdata
      (for (_array_element_3 _array_index_2) _playerdata
        (bind (_playerindex _playerconnected _playername _playermodel) (break `/Game/Core/Programming/Prototypes/GameData/BP_PlayerData` _array_element_2))
        (bind _int (`/Game/Core/Programming/Prototypes/GameData/GI_CORE_GameInstance.GetIntFromEnum` _currentgameinstance _playermodel))
        (bind (_playerindex_2 _playerconnected_2 _playername_2 _playermodel_2) (break `/Game/Core/Programming/Prototypes/GameData/BP_PlayerData` _array_element_3))
        (bind _int_2 (`/Game/Core/Programming/Prototypes/GameData/GI_CORE_GameInstance.GetIntFromEnum` _currentgameinstance _playermodel_2))
        (if (and (and _playerconnected _playerconnected_2) (== _int _int_2) (!= _array_index _array_index_2))
          (set `self.SameModel` true))))
    (if (`self.SameModel`)
      (`KismetSystemLibrary.PrintString` "players cannot have the same model")
      (else
        (`KismetSystemLibrary.PrintString` "CheckSuccessful")
        ;[1 1 1] Comment
        (`/Game/Core/Programming/Prototypes/Lobby/Widgets/WBP_CORE_LobbyMenu.StartGameCountdown` (`self.Lobby Widget`))))
    (else
      (`KismetSystemLibrary.PrintText` "Requires more than one player to start"))))

(event `ContinueToLevel`
  ;[0 0 0] SFX
  (bind _duration (`self.LobbyLockInVO`))
  (`KismetSystemLibrary.Delay` (+ _duration 0.5))
  ;[0 0 0] Load Level
  (`self.OpenNextLevel`))

(fn `LobbyLockInVO`
  (returns (Duration :type "Float (double-precision)"))
  (locals (SelectedSoundCue :type "SoundCue Object Reference"))
  (bind _asgi_core_game_instance (cast `/Game/Core/Programming/Prototypes/GameData/GI_CORE_GameInstance` (`GameplayStatics.GetGameInstance`)))
  (if (`/Game/Core/Programming/Prototypes/Test_Sai/PDA_GameInstanceSettings.TournamentMode` (`/Game/Core/Programming/Prototypes/GameData/GI_CORE_GameInstance.GameInstanceVariables` _asgi_core_game_instance))
    (bind _volobbyaudioatlas (`/Game/Core/Programming/Prototypes/GameData/GI_CORE_GameInstance.VOLobbyAudioAtlas` _asgi_core_game_instance))
    (bind _soundcue (`/Game/Audio/PDA_Core_AudioAtlas.GetSoundCue` _volobbyaudioatlas "NewEnumerator46"))
    (set `local.SelectedSoundCue` _soundcue)
    (else
      (bind _soundcue_2 (`/Game/Audio/PDA_Core_AudioAtlas.GetSoundCue` _volobbyaudioatlas "NewEnumerator44"))
      (set `local.SelectedSoundCue` _soundcue_2)))
  (`GameplayStatics.PlaySound2D` (`local.SelectedSoundCue`) 1.0 1.0 0.0 null null)
  (`/Engine/EditorBlueprintResources/StandardMacros.IsValid` (`local.SelectedSoundCue`)
    (:`Is Valid`
      (return (`SoundBase.Duration` (`local.SelectedSoundCue`))))
    (:`Is Not Valid`
      (return 0.0))))

(fn `OpenNextLevel`
  (bind _tournamentmode (`/Game/Core/Programming/Prototypes/Test_Sai/PDA_GameInstanceSettings.TournamentMode` (`/Game/Core/Programming/Prototypes/GameData/GI_CORE_GameInstance.GameInstanceVariables` (`self.CurrentGameInstance`))))
  (bind _asgi_core_game_instance (cast `/Game/Core/Programming/Prototypes/GameData/GI_CORE_GameInstance` (`GameplayStatics.GetGameInstance`)))
  (`/Game/Core/Programming/Prototypes/GameData/GI_CORE_GameInstance.StopMusic` _asgi_core_game_instance)
  (if _tournamentmode
    (`KismetSystemLibrary.PrintText` (`|FormatText` "The Game is in Tournament Mode: {TournamentMode}" _tournamentmode) true true (struct :`R` 1.0 :`G` 0.202734 :`B` 0.586872 :`A` 1.0))
    ;[1 1 1] Tournament
    (if (`KismetMathLibrary.RandomBool`)
      ;;[1 1 1] Starts With GameMode 1
      (`KismetSystemLibrary.PrintString` "Starting with GameMode 1")
      (`GameplayStatics.OpenLevelBySoftObjectPtr` "/Game/Core/Programming/Prototypes/Test_Sai/PreGameScreens/GM1_PreGameScreen.GM1_PreGameScreen")
      (else
        ;;[1 1 1] Starts with GameMode 2
        (`KismetSystemLibrary.PrintString` "Starting with GameMode 2")
        (`GameplayStatics.OpenLevelBySoftObjectPtr` "/Game/Core/Programming/Prototypes/Test_Sai/PreGameScreens/GM2_PreGameScreen.GM2_PreGameScreen")))
    (else
      (`GameplayStatics.OpenLevelBySoftObjectPtr` "/Game/Core/Programming/Prototypes/Test_Kellyn/Maps/LevelSelect.LevelSelect"))))

(fn `UserConstructionScript`)