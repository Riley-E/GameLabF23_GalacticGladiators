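; Voice-over announcer for the GM2 game mode, playing cues from the game instance's GM2 audio atlas through a single Speaker.
; After a short delay it binds to game-start events and FX manager callbacks.
; Start and death lines pass a ShouldSpeak gate of idle speaker, cooldown and random chance, while countdown interrupts current audio.
; End-game victory lines are disconnected, and super-star and player-kill handlers are empty.
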(event `self.ReceiveBeginPlay`
  (bind _gamemode (`self.GameMode`))
  (bind _fxmanager (`/Game/GameMode2/Programming/Gamemode/GM_GM2.FXManager` _gamemode))
  (`KismetSystemLibrary.Delay` 0.2)
  (`self.GatherVariables`)
  (add `/Game/GameMode2/Programming/Gamemode/GM_GM2.OnStartGame` _gamemode (delegate `OnStartGameVO`))
  (add `/Game/Systems/Blueprints/BP_FXEventManager.GM2_GameEnd` _fxmanager (delegate `OnGameEnd`))
  (add `/Game/Systems/Blueprints/BP_FXEventManager.GM2_PlayerDeath` _fxmanager (delegate `OnPlayerDeath`))
  (add `/Game/Systems/Blueprints/BP_FXEventManager.GM2_Countdown` _fxmanager (delegate `OnCountdown`))
  (add `/Game/Systems/Blueprints/BP_FXEventManager.GM2_LargeStarCollected` _fxmanager (delegate `OnSuperStarCollect`)))

(event `OnPlayerDeath`
  (params (Player :type "/Game/GameMode2/Programming/Movement/PC_GM2_Player Object Reference"))
  (`self.OnPlayerKill` Player))

(event `OnSuperStarCollect`
  (params (Star :type "/Game/GameMode2/Design/Powerups/BP_GM2_BigStar Object Reference")))

(event `OnStartGameVO`
  (`self.OnStartGame`)
  (for _array_element (`/Game/GameMode2/Programming/Gamemode/GM_GM2.Players` (`self.GameMode`))
    (add `/Game/GameMode2/Programming/Movement/PC_GM2_Player.OnPlayerKill` _array_element (delegate `OnPlayerKillVO`))))

(event `OnGameEnd`
  (`self.OnEndGame`))

(event `OnCountdown`
  (`self.Countdown`))

(event `OnPlayerKillVO`)

(event `SpawnSound`
  (params (Sound :type "SoundBase Object Reference"))
  (bind _speaker (`self.Speaker`))
  (set `self.CanSpeak` false)
  (`AudioComponent.SetSound` _speaker Sound)
  (`AudioComponent.Play` _speaker 0.0)
  (`KismetSystemLibrary.Delay` (+ (`SoundBase.Duration` Sound) (`self.DelayBetweenSpeakers`)))
  (set `self.CanSpeak` true))

(fn `Countdown`
  (`AudioComponent.Stop` (`self.Speaker`))
  (bind _soundcue (`/Game/Audio/PDA_Core_AudioAtlas.GetSoundCue` (`self.VOAudioAtlas`) "NewEnumerator53"))
  (`self.SpawnSound` _soundcue))

(fn `GatherVariables`
  (bind _asgi_core_game_instance (cast `/Game/Core/Programming/Prototypes/GameData/GI_CORE_GameInstance` (`GameplayStatics.GetGameInstance`)))
  (set `self.GameInstance` _asgi_core_game_instance)
  (bind _asgm_gm2 (cast `/Game/GameMode2/Programming/Gamemode/GM_GM2` (`GameplayStatics.GetGameMode`)))
  (set `self.GameMode` _asgm_gm2)
  (set `self.VOAudioAtlas` (`/Game/Core/Programming/Prototypes/GameData/GI_CORE_GameInstance.VOGM2AudioAtlas` (`self.GameInstance`))))

(fn `OnEndGame`
  (locals (PlayedSC :type "SoundCue Object Reference")))

(fn `OnPlayerKill`
  (params (KilledPlayer :type "/Game/GameMode2/Programming/Movement/PC_GM2_Player Object Reference"))
  (`self.ShouldSpeak`
    (:`Out`
      (bind _soundcue (`/Game/Audio/PDA_Core_AudioAtlas.GetSoundCue` (`self.VOAudioAtlas`) "NewEnumerator23"))
      (`self.SpawnSound` _soundcue))))

(fn `OnStartGame`
  (`self.ShouldSpeak`
    (:`Out`
      (bind _soundcue (`/Game/Audio/PDA_Core_AudioAtlas.GetSoundCue` (`self.VOAudioAtlas`) "NewEnumerator18"))
      (`self.SpawnSound` _soundcue))))

(fn `SuperStarCollect`
  (`KismetSystemLibrary.PrintString` "Super Star Voice Over Called")
  (`self.ShouldSpeak`
    (:`Out`
      (bind _soundcue (`/Game/Audio/PDA_Core_AudioAtlas.GetSoundCue` (`self.VOAudioAtlas`) "NewEnumerator54"))
      (`self.SpawnSound` _soundcue))))

(fn `UserConstructionScript`)