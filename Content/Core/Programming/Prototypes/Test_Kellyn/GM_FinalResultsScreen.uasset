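; Game mode for the final results screen, which shows the final ranking widget when play begins.
; BeginPlay sets the default menu input mapping context, spawns input pawns and displays WBP_FinalRankingScreen.
; DisplayWidget removes any visible current widget, adds the new WBP_GGWidgeBase-derived one to the viewport and passes it to each local BP_MenuInputReciever.
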(event `self.ReceiveBeginPlay`
  (set `self.DefaultIMC` "/Game/Core/Programming/Prototypes/Test_Kellyn/Input/IMC_Core_MenuDefault.IMC_Core_MenuDefault")
  (`self.SpawnInputPawns`)
  (`self.DisplayWidget` "/Game/Core/Programming/Prototypes/Test_Kellyn/Widgets/WBP_FinalRankingScreen.WBP_FinalRankingScreen_C"))

(fn `DisplayWidget`
  (params (Class :type "UserWidget Class Reference"))
  (bind _currentwidget (`self.CurrentWidget`))
  (`/Engine/EditorBlueprintResources/StandardMacros.IsValid` _currentwidget
    (:`Is Valid`
      (if (`Widget.IsVisible` _currentwidget)
        (`Widget.RemoveFromParent` _currentwidget)))
    (:`Is Not Valid`
      _))
  (bind _returnvalue (`|CreateWidget` Class))
  (bind _aswbp_ggwidge_base (cast `/Game/Core/Programming/Prototypes/Test_Sai/WBP_GGWidgeBase` _returnvalue))
  (bind _output_get (set `self.CurrentWidget` _aswbp_ggwidge_base))
  (`UserWidget.AddToViewport` _output_get 0)
  ;[1 1 1] Gives Each Input Reciever a Refernce to Main Menu Widget
  (for _array_element (`self.LocalInputs`)
    (bind _asbp_menu_input_reciever (cast `/Game/Core/Programming/Prototypes/Test_Kellyn/Input/BP_MenuInputReciever` _array_element))
    (`/Game/Core/Programming/Prototypes/Test_Kellyn/Input/BP_MenuInputReciever.SetWidgetReference` _asbp_menu_input_reciever (`self.CurrentWidget`))))

(fn `UserConstructionScript`
  (`parent.UserConstructionScript`))